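; Tank pawn Blueprint that hands its barrel, turret and tracks to aiming and movement components and links itself to its health bar widget on BeginPlay.
; Movement axes pass forward and turn intent to TankMovement, and the fire action calls TankAiming.
; Aim axes rotate an azimuth gimbal and spring arm for the third-person camera, scaled by frame time.
; Direct per-track throttle inputs are left unconnected.
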(event `self.ReceiveBeginPlay`
  (`TankAimingComponent.Initialize` (`self.TankAiming`) (`self.TankBarrel`) (`self.TankTurret`))
  (`TankMovementComponent.Initialize` (`self.TankMovement`) (`self.LeftTankTrack`) (`self.RightTankTrack`))
  (`self.InitializeHealthBarWidget`))

(event `InputAxis|AimAzimuth`
  (params (AxisValue :type "Float (single-precision)"))
  ;[1 1 1] 3rd Person Camera Input Binding
  (`SceneComponent.K2_AddLocalRotation` (`self.Azimuth Gimbal`) (`KismetMathLibrary.MakeRotator` 0.0 0.0 (* AxisValue (`GameplayStatics.GetWorldDeltaSeconds`) 100.0)) false false))

(event `InputAxis|Left Track Throttle`
  (params (AxisValue :type "Float (single-precision)"))
  ;[1 1 1] Movement Input Binding
)

(event `InputAxis|Right Track Throttle`
  (params (AxisValue :type "Float (single-precision)"))
  ;[1 1 1] Movement Input Binding
)

(event `InputAxis|AimElevation`
  (params (AxisValue :type "Float (single-precision)"))
  ;[1 1 1] 3rd Person Camera Input Binding
  (`SceneComponent.K2_AddLocalRotation` (`self.SpringArm`) (`KismetMathLibrary.MakeRotator` 0.0 (* AxisValue (`GameplayStatics.GetWorldDeltaSeconds`) 100.0)) false false))

(event `InputAxis|MoveForward`
  (params (AxisValue :type "Float (single-precision)"))
  ;[1 1 1] Movement Input Binding
  (`TankMovementComponent.IntendMoveForward` (`self.TankMovement`) AxisValue))

(event `InputAxis|TurnRight`
  (params (AxisValue :type "Float (single-precision)"))
  ;[1 1 1] Movement Input Binding
  (`TankMovementComponent.IntendTurnRight` (`self.TankMovement`) AxisValue))

(event `InputAction|Fire`
  (params (Key :type "Key Structure" :default "AnyKey"))
  ;[1 1 1] Tank Fire Input Binding
  (:`Pressed`
    (`TankAimingComponent.Fire` (`self.TankAiming`))))

(fn `InitializeHealthBarWidget`
  (bind _ashealth_bar_bp (cast `/Game/Blueprints/UI/HealthBar_BP` (`WidgetComponent.GetUserWidgetObject` (`self.HealthBar Component`))))
  (set `/Game/Blueprints/UI/HealthBar_BP.MyTank` self _ashealth_bar_bp))

(fn `UserConstructionScript`)